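; Custom Game Instance that holds the running points total and manages the records save file.
; LoadGame loads the save slot into a BP_CustomSaveGame reference, or creates and saves a new one when none exists.
; SaveGame writes a given points value into that object and saves it to the slot.
; IncrementPuntos adds to the running total and ClearInfo resets it to zero.
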(fn `ClearInfo`
  (set `self.TotalPuntos` 0))

(fn `IncrementPuntos`
  (params (Puntos :type Integer))
  (set `self.TotalPuntos` (+ Puntos (`self.TotalPuntos`))))

(fn `LoadGame`
  (bind _returnvalue (`GameplayStatics.DoesSaveGameExist` (`self.FileName`)))
  (if _returnvalue
    ;[1 1 1] Existe Records, lo cargamos en GameInstance
    (bind _returnvalue_2 (`GameplayStatics.LoadGameFromSlot` (`self.FileName`)))
    (bind _asbp_custom_save_game (cast `/Game/BP_CustomSaveGame` _returnvalue_2))
    (set `self.MyCustomSaveGame` _asbp_custom_save_game)
    (else
      ;[1 1 1] No existe un fichero Records
      (bind _returnvalue_3 (`GameplayStatics.CreateSaveGameObject` "/Game/BP_CustomSaveGame.BP_CustomSaveGame_C"))
      (bind _output_get (set `self.MyCustomSaveGame` _returnvalue_3))
      (`GameplayStatics.SaveGameToSlot` _output_get (`self.FileName`)))))

(fn `SaveGame`
  (params (`Total Puntos` :type Integer))
  (bind _mycustomsavegame (`self.MyCustomSaveGame`))
  (set `/Game/BP_CustomSaveGame.Puntos` `Total Puntos` _mycustomsavegame)
  (`GameplayStatics.SaveGameToSlot` _mycustomsavegame (`self.FileName`)))