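; BP_EnemyD is an enemy variant that extends a parent class with a diagonal MovementVector built from its right and forward vectors.
; Overlapping an actor tagged "Lateral2" toggles IsRight, and each flip from right to left shortens DelayShoot.
; Both toggle branches set the same left-forward vector, so the initial right-forward direction is not restored here.
; Movement and shooting themselves are not implemented in these graphs.
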(event `self.ReceiveBeginPlay`
  ;[1 1 1] Setup
  (`parent.ReceiveBeginPlay`)
  (set `self.MovementVector` (+ (`self.GetActorRightVector`) (`self.GetActorForwardVector`)))
  (set `self.IsRight` true))

(event `self.ReceiveActorBeginOverlap`
  (params (OtherActor :type "Actor Object Reference"))
  (bind _returnvalue (+ (* (`self.GetActorRightVector`) -1.0) (`self.GetActorForwardVector`)))
  ;[1 1 1] Overlap
  (`parent.ReceiveActorBeginOverlap` OtherActor)
  (if (`KismetArrayLibrary.Array_Contains` (`Actor.Tags` OtherActor) "Lateral2")
    (if (`self.IsRight`)
      (set `self.IsRight` false)
      (set `self.MovementVector` _returnvalue)
      (set `self.DelayShoot` (- (`self.DelayShoot`) 0.1))
      (else
        (set `self.IsRight` true)
        (set `self.MovementVector` _returnvalue)))))

(fn `UserConstructionScript`
  (`parent.UserConstructionScript`))