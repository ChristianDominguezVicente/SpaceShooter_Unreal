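; Base enemy for a space shooter that flies straight along its initial forward vector and fires ammo on a timer, both driven by Tick.
; Player overlap fires the OnEnemyDestroy dispatcher, updates game mode progress and game instance score, damages the player and plays explosion effects.
; The bound handler waits briefly, maybe spawns a random life, speed or shot power-up, then destroys the enemy.
; "Lateral" overlaps destroy it without rewards; the ammo-hit cast is unwired.
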(event `self.ReceiveBeginPlay`
  ;[1 1 1] Setup initial direction and Destroy Event
  (set `self.MovementVector` (`self.GetActorForwardVector`))
  (add `self.OnEnemyDestroy` (delegate `Destroyed_Event`)))

(event `Destroyed_Event`
  ;[1 1 1] Setup initial direction and Destroy Event
  (`KismetSystemLibrary.Delay` 0.2)
  (`self.SpawnPowerUp`)
  (`self.K2_DestroyActor`))

(event `self.ReceiveActorBeginOverlap`
  (params (OtherActor :type "Actor Object Reference"))
  (bind _tags (`Actor.Tags` OtherActor))
  ;[1 1 1] On Collision
  (if (`KismetArrayLibrary.Array_Contains` _tags "Player")
    (`self.OnEnemyDestroy`)
    (bind _asbp_ss_game_mode (cast `/Game/BP_SS_GameMode` (`GameplayStatics.GetGameMode`)))
    (`/Game/BP_SS_GameMode.EnemyDestroyed` _asbp_ss_game_mode)
    (`/Game/BP_SS_GameMode.AddProgress` _asbp_ss_game_mode (`self.Puntos`))
    (bind _asbp_space_s_character (cast `/Game/Players/BP_SpaceS_Character` OtherActor))
    (`/Game/Players/BP_SpaceS_Character.DamageActor` _asbp_space_s_character)
    (`GameplayStatics.SpawnEmitterAtLocation` "/Game/StarterContent/Particles/P_Explosion.P_Explosion" (`self.K2_GetActorLocation`))
    (`GameplayStatics.PlaySound2D` "/Game/StarterContent/Audio/Explosion01.Explosion01" 1.0 1.0 0.0 null null)
    (cast `/Game/BP_SS_GameMode` (`GameplayStatics.GetGameMode`))
    (bind _asbp_custom_game_instance (cast `/Game/BP_CustomGameInstance` (`GameplayStatics.GetGameInstance`)))
    (`/Game/BP_CustomGameInstance.IncrementPuntos` _asbp_custom_game_instance (`self.Puntos`))
    (elif (`KismetArrayLibrary.Array_Contains` _tags "Lateral")
      (`KismetSystemLibrary.Delay` 0.2)
      (`self.K2_DestroyActor`))))

(event `self.ReceiveTick`
  (params (DeltaSeconds :type "Float (single-precision)"))
  ;[1 1 1] Update Movement and Fire
  (`self.Move` DeltaSeconds)
  (bind _output_get (set `self.ShotCurrentTime` (+ DeltaSeconds (`self.ShotCurrentTime`))))
  (if (> _output_get (`self.DelayShoot`))
    (set `self.ShotCurrentTime` 0.0)
    (`self.Fire`)))

(fn `Fire`
  (bind _returnvalue (`|SpawnActorFromClass` (`self.Ammo`) (`SceneComponent.K2_GetComponentToWorld` (`self.FirePoint`)) "Undefined" "MultiplyWithRoot" null null))
  (`self.K2_SetActorRotation` _returnvalue (`self.K2_GetActorRotation`) false))

(fn `GetClassToSpawn`
  (returns (PowerUp :type "/Game/PowerUps/BP_Life Class Reference"))
  (return (select `int` (`KismetMathLibrary.RandomIntegerInRange` 0 2) :`0` "/Game/PowerUps/BP_Life.BP_Life_C" :`1` "/Game/PowerUps/BP_Speed.BP_Speed_C" :`2` "/Game/PowerUps/BP_Shoot.BP_Shoot_C" :!type "/Game/PowerUps/BP_Life Class Reference")))

(fn `Move`
  (params (DeltaTime :type "Float (double-precision)"))
  (`self.K2_SetActorLocation` (+ (`self.K2_GetActorLocation`) (* (* DeltaTime (`self.Speed`)) (`self.MovementVector`)))))

(fn `SpawnPowerUp`
  (if (<= (`KismetMathLibrary.RandomFloatInRange` 0.0 1.0) 0.5)
    (bind _powerup (`self.GetClassToSpawn`))
    (`|SpawnActorFromClass` _powerup (`SceneComponent.K2_GetComponentToWorld` (`self.FirePoint`)) "Undefined" "MultiplyWithRoot" null null)
    (return)))

(fn `UserConstructionScript`)