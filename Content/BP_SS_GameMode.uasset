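; Game mode for a space shooter that tracks score, difficulty and player death.
; Progress resets to zero on BeginPlay and grows through AddProgress.
; EnemyDestroyed counts kills and raises Level after every third one.
; PlayerDead casts the first player controller's HUD to BP_SpaceS_HUD and calls PlayerKilled on it.
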(event `self.ReceiveBeginPlay`
  ;[1 1 1] Establece los puntos iniciales
  (set `self.Progress` 0))

(event `self.ReceiveTick`
  (params (DeltaSeconds :type "Float (single-precision)")))

(event `PlayerDead`
  ;[1 1 1] Evento que se activa al morir el Player
  (bind _asbp_space_s_hud (cast `/Game/UI/BP_SpaceS_HUD` (`PlayerController.GetHUD` (`GameplayStatics.GetPlayerController` 0))))
  (`/Game/UI/BP_SpaceS_HUD.PlayerKilled` _asbp_space_s_hud))

(event `EnemyDestroyed`
  ;[1 1 1] Evento para controlar la dificultad
  (bind _output_get (set `self.EnemiesDestroyed` (+ (`self.EnemiesDestroyed`) 1)))
  (if (== (mod _output_get 3) 0)
    (set `self.Level` (+ (`self.Level`) 1))))

(event `AddProgress`
  (params (Puntos :type Integer))
  ;[1 1 1] Evento que añade puntos al HUD
  (set `self.Progress` (+ Puntos (`self.Progress`))))

(fn `UserConstructionScript`)