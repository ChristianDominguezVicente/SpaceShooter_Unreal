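; BP_SpaceS_Ammo is the space shooter projectile, moving itself every Tick in a pattern chosen by the GameMode's Progress.
; It flies straight at first, then in a sine wave, then along its Rotation vector for the triple shot.
; On overlap, actors tagged Lateral or Lateral2 remove it quietly after a short delay.
; Other actors, except PowerUps and Pawns, trigger an explosion effect and sound before it is destroyed.
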(event `self.ReceiveActorBeginOverlap`
  (params (OtherActor :type "Actor Object Reference"))
  (bind _tags (`Actor.Tags` OtherActor))
  (if (`KismetArrayLibrary.Array_Contains` _tags "Lateral")
    ;[1 1 1] Desaparecer Ammo
    (`KismetSystemLibrary.Delay` 0.2 :!label _label)
    (`self.K2_DestroyActor`)
    (elif (`KismetArrayLibrary.Array_Contains` _tags "Lateral2")
      (goto _label)
      (elif (not (`KismetArrayLibrary.Array_Contains` _tags "PowerUp"))
        ;[1 1 1] Colisión con enemigo
        (cast `Pawn` OtherActor
          (:`CastFailed`
            (`GameplayStatics.SpawnEmitterAtLocation` "/Game/StarterContent/Particles/P_Explosion.P_Explosion" (`self.K2_GetActorLocation`))
            (`GameplayStatics.PlaySound2D` "/Game/StarterContent/Audio/Explosion02.Explosion02" 1.0 1.0 0.0 null null)
            (`KismetSystemLibrary.Delay` 0.1)
            (`self.K2_DestroyActor`)))))))

(event `self.ReceiveBeginPlay`
  ;[1 1 1] Establecer el Game Mode
  (bind _asbp_ss_game_mode (cast `/Game/BP_SS_GameMode` (`GameplayStatics.GetGameMode`)))
  (set `self.GameMode` _asbp_ss_game_mode))

(event `self.ReceiveTick`
  (params (DeltaSeconds :type "Float (single-precision)"))
  (bind _progress (`/Game/BP_SS_GameMode.Progress` (`self.GameMode`)))
  (if (>= _progress 100)
    (if (>= _progress 200)
      ;[1 1 1] Disparo Triple
      (`self.K2_SetActorLocation` (+ (`self.K2_GetActorLocation`) (* (`self.Rotation`) (* DeltaSeconds (`self.Speed`)))))
      (else
        ;[1 1 1] Disparo Ondulante
        (bind _output_get (set `self.Time` (+ DeltaSeconds (`self.Time`))))
        (`self.K2_SetActorLocation` (+ (`self.K2_GetActorLocation`) (* (`self.GetActorForwardVector`) (* DeltaSeconds (`self.Speed`))) (* (`self.GetActorRightVector`) (* (`self.Amplitud`) (`KismetMathLibrary.Sin` (* _output_get (`self.Frecuencia`))) (`self.Direction`)))))))
    (else
      ;[1 1 1] Disparo Recto
      (`self.K2_SetActorLocation` (+ (`self.K2_GetActorLocation`) (* (`self.GetActorForwardVector`) (* DeltaSeconds (`self.Speed`))))))))

(fn `UserConstructionScript`)