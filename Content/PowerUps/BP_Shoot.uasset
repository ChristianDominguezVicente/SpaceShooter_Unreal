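; BP_Shoot is a power-up actor that grants the player's ship its shoot ability on contact.
; Overlapping a Player-tagged actor without the Ammo tag calls OnLifeDestroy, then ShootActor on the BP_SpaceS_Character, with an emitter and sound.
; Overlapping a non-player actor tagged Lateral destroys the pickup after a short delay, clearing it once it leaves the screen.
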(event `self.ReceiveActorBeginOverlap`
  (params (OtherActor :type "Actor Object Reference"))
  (bind _tags (`Actor.Tags` OtherActor))
  (if (`KismetArrayLibrary.Array_Contains` _tags "Player")
    ;[1 1 1] Overlap con Player
    (if (not (`KismetArrayLibrary.Array_Contains` _tags "Ammo"))
      (`self.OnLifeDestroy`)
      (bind _asbp_space_s_character (cast `/Game/Players/BP_SpaceS_Character` OtherActor))
      (`/Game/Players/BP_SpaceS_Character.ShootActor` _asbp_space_s_character)
      (`GameplayStatics.SpawnEmitterAtLocation` null (`self.K2_GetActorLocation`))
      (`GameplayStatics.PlaySound2D` "/Engine/VREditor/Sounds/UI/Camera_Shutter.Camera_Shutter" 1.0 1.0 0.0 null null))
    (else
      ;[1 1 1] Desaparece de la pantalla
      (if (`KismetArrayLibrary.Array_Contains` _tags "Lateral")
        (`KismetSystemLibrary.Delay` 0.2)
        (`self.K2_DestroyActor`)))))

(fn `UserConstructionScript`
  (`parent.UserConstructionScript`))